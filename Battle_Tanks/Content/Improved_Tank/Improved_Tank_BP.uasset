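; Player-controllable tank pawn that drives on two tracks, aims a turret and barrel, and fires.
; On BeginPlay it hands the barrel and turret to TankAiming and both tracks to TankMovement, then assigns their meshes.
; Input axes feed movement intents and rotate an azimuth gimbal and spring arm for camera look, while Fire calls TankAiming.
; A track physical-material override is present but never runs.
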(event `self.ReceiveBeginPlay`
  (`TankAimingComponent.Initialize` (`self.TankAiming`) (`self.TankBarrel`) (`self.TankTurret`))
  (`TankMovementComponent.Initialize` (`self.TankMovement`) (`self.Left Track`) (`self.Right Track`))
  (`StaticMeshComponent.SetStaticMesh` (`self.Left Track`) "/Game/Improved_Tank/improved_tank_fbx_Track.improved_tank_fbx_Track")
  (`StaticMeshComponent.SetStaticMesh` (`self.Right Track`) "/Game/Improved_Tank/improved_tank_fbx_Track.improved_tank_fbx_Track")
  (`StaticMeshComponent.SetStaticMesh` (`self.TankTurret`) "/Game/Improved_Tank/improved_tank_fbx_Turret.improved_tank_fbx_Turret")
  (`StaticMeshComponent.SetStaticMesh` (`self.TankBarrel`) "/Game/Improved_Tank/improved_tank_fbx_Barrel.improved_tank_fbx_Barrel"))

(event `InputAxis|MoveForward`
  (params (AxisValue :type "Float (single-precision)"))
  ;[1 1 1] Movement
  (`TankMovementComponent.IntendMoveForward` (`self.TankMovement`) AxisValue))

(event `InputAxis|AimAzimuth`
  (params (AxisValue :type "Float (single-precision)"))
  ;[1 1 1] Camera Input Binding
  (`SceneComponent.K2_AddLocalRotation` (`self.AzimuthGimbal`) (`KismetMathLibrary.MakeRotator` 0.0 0.0 AxisValue) false false))

(event `InputAxis|TurnRight`
  (params (AxisValue :type "Float (single-precision)"))
  ;[1 1 1] Movement
  (`TankMovementComponent.IntendTurnRight` (`self.TankMovement`) AxisValue))

(event `InputAxis|AimElevation`
  (params (AxisValue :type "Float (single-precision)"))
  ;[1 1 1] Camera Input Binding
  (`SceneComponent.K2_AddLocalRotation` (`self.SpringArm`) (`KismetMathLibrary.MakeRotator` 0.0 AxisValue) false false))

(event `InputAction|Fire`
  (params (Key :type "Key Structure"))
  ;[1 1 1] Movement
  (:`Pressed`
    (`TankAimingComponent.Fire` (`self.TankAiming`))))

(fn `UserConstructionScript`)